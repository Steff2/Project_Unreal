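; Cube spawner for the FullRoomSmall scene that runs a timed capture of position and collision data.
; On BeginPlay it spawns five Cube_BP actors at once at the same fixed transform.
; It finds the PositionAndCollision actor through GetAllActorsOfClass, sets its scene name and a blank spawn rate for export.
; After a ten-second delay it calls that actor's collision and position exports, printing a confirmation after each.
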(event `self.ReceiveBeginPlay`
  (for _ (range 5)
    (`|SpawnActorFromClass` "/Game/Blueprints/Cube_BP.Cube_BP_C" (`KismetMathLibrary.MakeTransform` (0.0 -20.0 50.0)) "Undefined" "OverrideRootScale" null null))
  (bind _outactors (`GameplayStatics.GetAllActorsOfClass` "/Game/Blueprints/PositionAndCollision.PositionAndCollision_C")) ; Workaround to get function from other blueprint
  (bind _output (`|GetArrayItem` _outactors))
  (set `/Game/Blueprints/PositionAndCollision.sceneName` "FullRoomSmall" _output) ; set scene name for export
  (set `/Game/Blueprints/PositionAndCollision.spawnRate` "" _output) ; set spawn rate for export
  (bind _outactors_2 (`GameplayStatics.GetAllActorsOfClass` "/Game/Blueprints/PositionAndCollision.PositionAndCollision_C")) ; Workaround to get function from other blueprint
  (`KismetSystemLibrary.Delay` 10.0) ; exit time for the scene
  (bind _output_2 (`|GetArrayItem` _outactors_2))
  (`/Game/Blueprints/PositionAndCollision.ExportCol` _output_2) ; call the export collision function
  (`KismetSystemLibrary.PrintString` "Exported Col")
  (`/Game/Blueprints/PositionAndCollision.ExportPos` _output_2) ; call the export position function
  (`KismetSystemLibrary.PrintString` "Exported Pos"))

(fn `UserConstructionScript`)