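; PositionAndCollision is a data logger that exports cube position and collision records to text files in a hard-coded MATLAB data directory.
; ExportPos loops through Positions, splits out each cube's identifier and saves the entry to a position file named after it.
; ExportCol saves the whole Collisions array to one file.
; Both build the folder path from SceneName, SpawnRate and Testsatz, print it and write via SaveArrayText.
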(fn `ExportCol`
  (bind _returnvalue (`KismetStringLibrary.Concat_StrStr` "f:\\MATLAB\\Data\\UnrealEngine4\\" (`self.sceneName`) (`self.spawnRate`) (`self.Testsatz`)))
  (`KismetSystemLibrary.PrintString` _returnvalue)
  (`ExportManager.SaveArrayText` _returnvalue "data_Collision.txt" (`self.Collisions`)))

(fn `ExportPos`
  (bind _returnvalue (`KismetStringLibrary.Concat_StrStr` "f:\\MATLAB\\Data\\UnrealEngine4\\" (`self.sceneName`) (`self.spawnRate`) (`self.Testsatz`)))
  (`KismetSystemLibrary.PrintString` _returnvalue)
  (for _array_element (`self.Positions`)
    (`ExportManager.SaveArrayText` _returnvalue (`KismetStringLibrary.Concat_StrStr` "data_Position_" (`KismetStringLibrary.Split` _array_element " ") ".txt") (`|MakeArray` _array_element))))

(fn `UserConstructionScript`)