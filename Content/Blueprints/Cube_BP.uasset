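; Cube actor Blueprint that logs its movement and collisions to a PositionAndCollision actor, found with GetAllActorsOfClass as a cross-Blueprint workaround.
; Every tick, it appends its name, cube location and game time to that actor's Positions array.
; On component hit, a 0.15-second delay precedes adding both objects' names, locations, their distance and the time to Collisions.
; Both entries are concatenated strings with X/Y/Z axis labels stripped.
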(event `self.ReceiveTick`
  (params (DeltaSeconds :type "Float (single-precision)"))
  (bind _outactors (`GameplayStatics.GetAllActorsOfClass` "/Game/Blueprints/PositionAndCollision.PositionAndCollision_C")) ; Workaround to get function from other blueprint
  (`KismetArrayLibrary.Array_Add` (`/Game/Blueprints/PositionAndCollision.Positions` (`|GetArrayItem` _outactors)) (`KismetStringLibrary.Replace` (`KismetStringLibrary.Replace` (`KismetStringLibrary.Replace` (`KismetStringLibrary.Concat_StrStr` (`KismetStringLibrary.Conv_ObjectToString` self) " " (`KismetStringLibrary.Conv_VectorToString` (`SceneComponent.K2_GetComponentLocation` (`self.Cube`))) " " (`KismetStringLibrary.Conv_DoubleToString` (`KismetSystemLibrary.GetGameTimeInSeconds`))) "Y=") "X=") "Z=")) ; Add new entry to position array
)

(event `self.Cube.OnComponentHit`
  (params (HitComponent :type "PrimitiveComponent Object Reference") (OtherActor :type "Actor Object Reference") (OtherComp :type "PrimitiveComponent Object Reference") (NormalImpulse :type "Vector Structure") (Hit :type "HitResult Structure (by ref)"))
  (bind _returnvalue (`SceneComponent.K2_GetComponentLocation` OtherComp))
  (bind _returnvalue_2 (`SceneComponent.K2_GetComponentLocation` HitComponent))
  (bind _outactors (`GameplayStatics.GetAllActorsOfClass` "/Game/Blueprints/PositionAndCollision.PositionAndCollision_C")) ; Workaround to get function from other blueprint
  (`KismetSystemLibrary.Delay` 0.15) ; delay before adding entry
  (`KismetArrayLibrary.Array_Add` (`/Game/Blueprints/PositionAndCollision.Collisions` (`|GetArrayItem` _outactors)) (`KismetStringLibrary.Replace` (`KismetStringLibrary.Replace` (`KismetStringLibrary.Replace` (`KismetStringLibrary.Concat_StrStr` (`KismetStringLibrary.Conv_ObjectToString` self) " " (`KismetStringLibrary.Conv_VectorToString` _returnvalue_2) " " (`KismetStringLibrary.Conv_ObjectToString` OtherActor) " " (`KismetStringLibrary.Conv_VectorToString` _returnvalue) " " (`KismetStringLibrary.Conv_DoubleToString` (`KismetMathLibrary.Vector_Distance` _returnvalue_2 _returnvalue)) " " (`KismetStringLibrary.Conv_DoubleToString` (`KismetSystemLibrary.GetGameTimeInSeconds`))) "Y=") "X=") "Z=")) ; Add new entry to collision array
)

(fn `UserConstructionScript`)