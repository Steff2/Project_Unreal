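; Spawner actor for the FullRoom scene that creates Cube_BP actors and triggers a timed collision and position data export.
; Each Tick spawns a cube at a fixed transform, so the actor's tick interval acts as the spawn rate.
; BeginPlay passes the scene name and spawn-rate label to the first PositionAndCollision actor found, then calls its two export functions after a fixed delay.
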(event `self.ReceiveBeginPlay`
  (bind _outactors (`GameplayStatics.GetAllActorsOfClass` "/Game/Blueprints/PositionAndCollision.PositionAndCollision_C")) ; Workaround to get function from other blueprint
  (bind _output (`|GetArrayItem` _outactors))
  (set `/Game/Blueprints/PositionAndCollision.sceneName` "FullRoom" _output) ; set the scene name
  (set `/Game/Blueprints/PositionAndCollision.spawnRate` (`KismetStringLibrary.Concat_StrStr` "\\Spawnrate" "_" (`KismetStringLibrary.Conv_DoubleToString` (`self.GetActorTickInterval`))) _output) ; set the spawn rate for export
  (bind _outactors_2 (`GameplayStatics.GetAllActorsOfClass` "/Game/Blueprints/PositionAndCollision.PositionAndCollision_C")) ; Workaround to get function from other blueprint
  (`KismetSystemLibrary.Delay` 40.0) ; exit time for the scene
  (bind _output_2 (`|GetArrayItem` _outactors_2))
  (`/Game/Blueprints/PositionAndCollision.ExportCol` _output_2) ; call the export collision function
  (`KismetSystemLibrary.PrintString` "Exported Col")
  (`/Game/Blueprints/PositionAndCollision.ExportPos` _output_2) ; call the export position function
  (`KismetSystemLibrary.PrintString` "Exported Pos"))

(event `self.ReceiveTick`
  (params (DeltaSeconds :type "Float (single-precision)"))
  (`|SpawnActorFromClass` "/Game/Blueprints/Cube_BP.Cube_BP_C" (`KismetMathLibrary.MakeTransform` (40.0 80.0 30.0)) "Undefined" "OverrideRootScale" null null) ; Spawn Cube with specific blueprint every tick
)

(fn `UserConstructionScript`)