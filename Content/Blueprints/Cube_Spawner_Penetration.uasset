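; Cube_Spawner_Penetration is a scene driver for a "Penetration" test that exports position and collision data from a PositionAndCollision actor.
; On BeginPlay it finds that actor through GetAllActorsOfClass, a workaround for calling another Blueprint, and sets its scene name and spawn rate for export.
; After a fixed delay serving as the scene's exit time, it calls the actor's collision and position export functions, printing a message after each.
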(event `self.ReceiveBeginPlay`
  (bind _outactors (`GameplayStatics.GetAllActorsOfClass` "/Game/Blueprints/PositionAndCollision.PositionAndCollision_C")) ; Workaround to get function from other blueprint
  (bind _output (`|GetArrayItem` _outactors))
  (set `/Game/Blueprints/PositionAndCollision.sceneName` "Penetration" _output) ; set scene name for export
  (set `/Game/Blueprints/PositionAndCollision.spawnRate` "\\" _output) ; set spawn rate for export
  (bind _outactors_2 (`GameplayStatics.GetAllActorsOfClass` "/Game/Blueprints/PositionAndCollision.PositionAndCollision_C")) ; Workaround to get function from other blueprint
  (`KismetSystemLibrary.Delay` 5.0) ; exit time for the scene
  (bind _output_2 (`|GetArrayItem` _outactors_2))
  (`/Game/Blueprints/PositionAndCollision.ExportCol` _output_2) ; call the export collision function
  (`KismetSystemLibrary.PrintString` "Exported Col")
  (`/Game/Blueprints/PositionAndCollision.ExportPos` _output_2) ; call the export position function
  (`KismetSystemLibrary.PrintString` "Exported Pos"))

(fn `UserConstructionScript`)